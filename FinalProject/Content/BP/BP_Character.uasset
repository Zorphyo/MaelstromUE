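; Player character handling Enhanced Input movement and look, health, death, interaction and pause menu.
; BeginPlay fades the camera and creates the HUD, then after a delay opens dialogue, adds input mapping and creates the interact prompt.
; A per-tick mesh-forward trace toggles that prompt and custom-depth highlighting on the first interface actor found, not necessarily the hit one.
; Interact messages overlapping actors; damage updates the HUD and disables movement at zero health.
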(event Custom|Death
  (bind _charactermovement (Variables|Character|GetCharacterMovement))
  ;[1 1 1] Update Health
  (Variables|Default|SetIsDead true)
  (Components|Movement|StopMovementImmediately _charactermovement)
  (Pawn|Components|CharacterMovement|DisableMovement _charactermovement))

(event Input|EnhancedActionEvents|EnhancedInputActionIA_Locomotion
  (params (ActionValue :type Float%20%28double-precision%29) (ElapsedSeconds :type Float%20%28double-precision%29) (TriggeredSeconds :type Float%20%28double-precision%29) (InputAction :type Input%20Action%20Object%20Reference :default "/Game/BP/UI/IO/IA_Locomotion.IA_Locomotion"))
  ;[1 1 1] Basic Input
  (:Triggered
    (if (not (Variables|Default|GetInInventory))
      (Pawn|Input|AddMovementInput (Transformation|GetActorForwardVector) ActionValue false))))

(event Input|EnhancedActionEvents|EnhancedInputActionIA_LookH
  (params (ActionValue :type Float%20%28double-precision%29) (ElapsedSeconds :type Float%20%28double-precision%29) (TriggeredSeconds :type Float%20%28double-precision%29) (InputAction :type Input%20Action%20Object%20Reference :default "/Game/BP/UI/IO/IA_LookH.IA_LookH"))
  ;[1 1 1] Basic Input
  (:Triggered
    (if (not (Variables|Default|GetIsDead))
      (Pawn|Input|AddControllerYawInput ActionValue))))

(event Input|EnhancedActionEvents|EnhancedInputActionIA_Strafe
  (params (ActionValue :type Float%20%28double-precision%29) (ElapsedSeconds :type Float%20%28double-precision%29) (TriggeredSeconds :type Float%20%28double-precision%29) (InputAction :type Input%20Action%20Object%20Reference :default "/Game/BP/UI/IO/IA_Strafe.IA_Strafe"))
  ;[1 1 1] Basic Input
  (:Triggered
    (if (not (Variables|Default|GetInInventory))
      (Pawn|Input|AddMovementInput (Transformation|GetActorRightVector) ActionValue false))))

(event Input|EnhancedActionEvents|EnhancedInputActionIA_LookV
  (params (ActionValue :type Float%20%28double-precision%29) (ElapsedSeconds :type Float%20%28double-precision%29) (TriggeredSeconds :type Float%20%28double-precision%29) (InputAction :type Input%20Action%20Object%20Reference :default "/Game/BP/UI/IO/IA_LookV.IA_LookV"))
  ;[1 1 1] Basic Input
  (:Triggered
    (if (not (Variables|Default|GetIsDead))
      (Pawn|Input|AddControllerPitchInput ActionValue))))

(event Input|EnhancedActionEvents|EnhancedInputActionIA_Pause
  (params (ActionValue :type Boolean) (ElapsedSeconds :type Float%20%28double-precision%29) (TriggeredSeconds :type Float%20%28double-precision%29) (InputAction :type Input%20Action%20Object%20Reference :default "/Game/BP/UI/IO/IA_Pause.IA_Pause"))
  (bind _returnvalue (Game|GetPlayerController 0))
  ;[1 1 1] Pause Game
  (:Started
    (bind _returnvalue_2 (UserInterface|CreateWidget "/Game/BP/UI/PauseMenu.PauseMenu_C"))
    (UserInterface|Viewport|AddtoViewport _returnvalue_2 0)
    (Variables|/Script/Engine.PlayerController|SetbShowMouseCursor _returnvalue true)
    (Input|SetInputModeUIOnly _returnvalue 0 "DoNotLock" false)
    (Game|SetGamePaused false)))

(event Game|Damage|EventAnyDamage
  (params (Damage :type Float%20%28single-precision%29) (DamageType :type Damage%20Type%20Object%20Reference) (InstigatedBy :type Controller%20Object%20Reference) (DamageCauser :type Actor%20Object%20Reference))
  ;[1 1 1] Update Health
  (if (not (Variables|Default|GetInInventory))
    (if (not (Variables|Default|GetIsDead))
      (bind _output_get (Variables|Default|SetCurrentHealth (Math|Float|Clamp(Float) (- (Variables|Default|GetCurrentHealth) Damage) 0.0 (Variables|Default|GetMaxHealth))))
      (Default|UpdateHealthUI (Variables|Default|GetWB_Main) _output_get (Variables|Default|GetMaxHealth))
      (if (== (Variables|Default|GetCurrentHealth) 0.0)
        (CallFunction|Death)))))

(event EventTick
  (params (DeltaSeconds :type Float%20%28single-precision%29))
  (bind _interactuiwidget (Variables|Default|GetInteractUIWidget))
  (bind _interactuiwidget_2 (Variables|Default|GetInteractUIWidget))
  (bind _mesh (Variables|Character|GetMesh))
  (bind _returnvalue (Transformation|GetWorldLocation _mesh))
  (bind _returnvalue_2 (UserInterface|Viewport|IsinViewport _interactuiwidget_2))
  ;[1 1 1] Interact UI
  (Variables|Default|GetInteractUIWidget
    (:then
      (bind (_outhit _returnvalue_3) (Collision|LineTraceByChannel _returnvalue (+ _returnvalue (* (Math|Vector|GetForwardVector _mesh) 2e+02)) "TraceTypeQuery1" false 0 "None"))
      (if _returnvalue_3
        (if (Utilities|DoesObjectImplementInterface (.HitActor (Collision|BreakHitResult _outhit)) "/Game/BP/InteractInterface.InteractInterface_C")
          (if (not _returnvalue_2)
            (UserInterface|Viewport|AddtoViewport _interactuiwidget 0)
            ;[1 1 1] Highlight Interactable Items
            (bind _outactors (Actor|GetAllActorswithInterface "/Game/BP/InteractInterface.InteractInterface_C"))
            (Rendering|SetRenderCustomDepth (Actor|GetComponentsByClass (Utilities|Array|Get(acopy) _outactors) "/Script/Engine.PrimitiveComponent") true))
          (else
            (if _returnvalue_2 :!label _label
              (Widget|RemovefromParent _interactuiwidget)
              (bind _outactors_2 (Actor|GetAllActorswithInterface "/Game/BP/InteractInterface.InteractInterface_C"))
              (if (not (Utilities|Array|IsEmpty _outactors_2))
                (Rendering|SetRenderCustomDepth (Actor|GetComponentsByClass (Utilities|Array|Get(acopy) _outactors_2) "/Script/Engine.PrimitiveComponent") false)))))
        (else
          (goto _label))))
    (:else)))

(event EventBeginPlay
  ;[1 1 1] Camera Fade
  (CameraFades|StartCameraFade :self (Game|GetPlayerCameraManager 0) :FromAlpha 1.0 :Duration 4.0 :bShouldFadeAudio true :bHoldWhenFinished true)
  ;[1 1 1] UI
  (bind _returnvalue (UserInterface|CreateWidget "/Game/BP/UI/WB_Main.WB_Main_C" (Game|GetPlayerController 0)))
  (bind _output_get (Variables|Default|SetWB_Main _returnvalue))
  (UserInterface|Viewport|AddtoViewport _output_get 0)
  (bind _output_get_2 (Variables|Default|SetCurrentHealth (Variables|Default|GetMaxHealth)))
  (Default|UpdateHealthUI (Variables|Default|GetWB_Main) _output_get_2 (Variables|Default|GetMaxHealth))
  ;[1 1 1] Establish IMC Mapping
  (Utilities|FlowControl|Delay 4.0)
  ;[1 1 1] Opening Dialogue
  (Utilities|FlowControl|Sequence
    (:then_0
      (bind _returnvalue_2 (UserInterface|CreateWidget "/Game/BP/UI/WB_Dialogue.WB_Dialogue_C"))
      (UserInterface|Viewport|AddtoViewport _returnvalue_2 0))
    (:then_1
      (Utilities|FlowControl|Sequence
        (:then_0
          (Input|AddMappingContext (PlayerController|LocalPlayerSubsystems|GetEnhancedInputLocalPlayerSubsystem (Game|GetPlayerController 0)) "/Game/BP/UI/IO/IMC_BaseCharacter.IMC_BaseCharacter" 0 "(bIgnoreAllPressedKeysUntilRelease=True,bForceImmediately=False)"))
        (:then_1
          ;[1 1 1] Interact UI
          (bind _returnvalue_3 (UserInterface|CreateWidget "/Game/BP/UI/InteractUI.InteractUI_C"))
          (Variables|Default|SetInteractUIWidget _returnvalue_3))))))

(event Input|ActionEvents|InputActionInteract
  (params (Key :type Key%20Structure :default "None"))
  ;[1 1 1] Interaction/Pickup
  (:Pressed
    (bind _array_element (Utilities|Array|ForEachLoopwithBreak (Collision|GetOverlappingActors "/Script/Engine.Actor" :!class /Script/Engine.Actor))
      (:LoopBody
        (if (Utilities|DoesObjectImplementInterface _array_element "/Game/BP/InteractInterface.InteractInterface_C")
          (bind _item (Class|InteractInterface|Interact(Message) _array_element))
          (bind _output_get (Variables|Default|SetHeld%20Item _item))
          (Development|PrintString _output_get))))))

(fn ConstructionScript)