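; BP_PickUpSocket is an interactable socket wrench pickup that swaps places with the BP_PickUpWrench pickup when taken.
; Sphere overlap by a Character toggles custom depth on the mesh to highlight it.
; Interact plays a sound at world origin, sets the interactor's EquippedItem mesh and returns the item name.
; SwapWrenches hides and disables this pickup instead of destroying it, then reveals and re-enables the first BP_PickUpWrench found.
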(event OnComponentEndOverlap(Sphere)
  (params (OverlappedComponent :type Primitive%20Component%20Object%20Reference) (OtherActor :type Actor%20Object%20Reference) (OtherComp :type Primitive%20Component%20Object%20Reference) (OtherBodyIndex :type Integer))
  ;[1 1 1] Highlight Item
  (Utilities|Casting|CastToCharacter OtherActor)
  (Rendering|SetRenderCustomDepth (Variables|Default|GetStaticMesh) false))

(event OnComponentBeginOverlap(Sphere)
  (params (OverlappedComponent :type Primitive%20Component%20Object%20Reference) (OtherActor :type Actor%20Object%20Reference) (OtherComp :type Primitive%20Component%20Object%20Reference) (OtherBodyIndex :type Integer) (bFromSweep :type Boolean) (SweepResult :type Hit%20Result%20Structure%20%28by%20ref%29))
  ;[1 1 1] Highlight Item
  (Utilities|Casting|CastToCharacter OtherActor)
  (Rendering|SetRenderCustomDepth (Variables|Default|GetStaticMesh) true))

(event Custom|Swap%20Wrenches
  (bind _staticmesh (Variables|Default|GetStaticMesh))
  (bind _sphere (Variables|Default|GetSphere))
  ;[1 1 1] Swap Wrenches When Picking One Up
  (Collision|SetCollisionEnabled _staticmesh "NoCollision")
  (Collision|SetCollisionEnabled _sphere "NoCollision")
  (Development|SetHiddeninGame _staticmesh true true)
  (Development|SetHiddeninGame _sphere true true)
  (bind _returnvalue (Actor|GetActorOfClass "/Game/BP/BP_PickUpWrench.BP_PickUpWrench_C"))
  (Collision|SetCollisionEnabled (Variables|/Game/BP/BP_PickUpWrench.BP_PickUpWrench_C|GetStaticMesh _returnvalue) "QueryAndPhysics")
  (Collision|SetCollisionEnabled (Variables|/Game/BP/BP_PickUpWrench.BP_PickUpWrench_C|GetSphere _returnvalue) "QueryAndPhysics")
  (Development|SetHiddeninGame (Variables|/Game/BP/BP_PickUpWrench.BP_PickUpWrench_C|GetStaticMesh _returnvalue) false true))

(event EventBeginPlay)

(event Collision|EventActorBeginOverlap
  (params (OtherActor :type Actor%20Object%20Reference)))

(event EventTick
  (params (DeltaSeconds :type Float%20%28single-precision%29)))

(fn ConstructionScript)

(fn Interact
  (params (Interactor :type BP%20First%20Person%20Character%20Object%20Reference))
  ;[1 1 1] Pick Up Socket Wrench
  (Audio|PlaySoundatLocation "/Game/Sound/Miscellaneous/PickupWrench.PickupWrench" "0, 0, 0" "0, 0, 0" 1.0 1.0 0.0 0 0 0 0)
  (CallFunction|SwapWrenches)
  (Components|StaticMesh|SetStaticMesh (Variables|/Game/FirstPerson/Blueprints/BP_FirstPersonCharacter.BP_FirstPersonCharacter_C|GetEquippedItem Interactor) (Variables|Default|GetItemModel self))
  (return "Socket Wrench"))