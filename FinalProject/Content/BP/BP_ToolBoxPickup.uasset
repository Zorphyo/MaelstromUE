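; Pickup actor for a tool box item that a character can equip through an Interact function.
; The construction script sets the mesh from ItemModel, and a sphere overlap with a Character toggles custom depth on the mesh, presumably for highlighting.
; Interact copies ItemModel onto the interactor's EquippedItem mesh and destroys the pickup after a brief delay.
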(event OnComponentEndOverlap(Sphere)
  (params (OverlappedComponent :type Primitive%20Component%20Object%20Reference) (OtherActor :type Actor%20Object%20Reference) (OtherComp :type Primitive%20Component%20Object%20Reference) (OtherBodyIndex :type Integer))
  (Utilities|Casting|CastToCharacter OtherActor)
  (Rendering|SetRenderCustomDepth (Variables|Default|GetStaticMesh) false))

(event OnComponentBeginOverlap(Sphere)
  (params (OverlappedComponent :type Primitive%20Component%20Object%20Reference) (OtherActor :type Actor%20Object%20Reference) (OtherComp :type Primitive%20Component%20Object%20Reference) (OtherBodyIndex :type Integer) (bFromSweep :type Boolean) (SweepResult :type Hit%20Result%20Structure%20%28by%20ref%29))
  (Utilities|Casting|CastToCharacter OtherActor)
  (Rendering|SetRenderCustomDepth (Variables|Default|GetStaticMesh) true))

(event Custom|Destroy%20Item
  (Utilities|FlowControl|Delay 0.05)
  (Actor|DestroyActor))

(event EventBeginPlay)

(event Collision|EventActorBeginOverlap
  (params (OtherActor :type Actor%20Object%20Reference)))

(event EventTick
  (params (DeltaSeconds :type Float%20%28single-precision%29)))

(fn ConstructionScript
  (Components|StaticMesh|SetStaticMesh (Variables|Default|GetStaticMesh) (Variables|Default|GetItemModel)))

(fn Interact
  (params (Interactor :type BP%20First%20Person%20Character%20Object%20Reference))
  (CallFunction|DestroyItem)
  (Components|StaticMesh|SetStaticMesh (Variables|/Game/FirstPerson/Blueprints/BP_FirstPersonCharacter.BP_FirstPersonCharacter_C|GetEquippedItem Interactor) (Variables|Default|GetItemModel self))
  (return ""))